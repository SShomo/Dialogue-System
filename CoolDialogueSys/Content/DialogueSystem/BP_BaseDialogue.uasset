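; BP_BaseDialogue is a base dialogue Blueprint that serves lines of text one at a time.
; A Dialogue struct holds the line array and the current index.
; GetNextDialogue returns the line at the index and advances it, or returns empty text with HasFinished set once the lines run out.
; The ResetDialogue event sets the index back to the start so the conversation can replay.
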(event `/Game/DialogueSystem/DialogueInterface.ResetDialogue`
  (`|VariableSetRef` (`.DialogueIndex_12_5D8B952442137F1A875C9EA824FBAEB4` (break `/Game/DialogueSystem/Dialogue` (`self.Dialogue`)))))

(fn `GetNextDialogue`
  (returns (Text :type String) (hasFinished :type Boolean))
  (bind (_dialogue _dialogueindex) (break `/Game/DialogueSystem/Dialogue` (`self.Dialogue`)))
  (if (< _dialogueindex (`KismetArrayLibrary.Array_Length` _dialogue))
    (`/Engine/EditorBlueprintResources/StandardMacros.IncrementInt` _dialogueindex
      (:`  `
        (return (`|GetArrayItem` _dialogue (- _dialogueindex 1)) false)))
    (else
      (return "" true))))

(fn `UserConstructionScript`)