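; BP_RepeatingDialogue is a dialogue Blueprint that cycles endlessly through its lines.
; GetNextDialogue returns the line at the current index and advances it, calling ResetDialogue first once the index reaches the end of the array.
; It always reports HasFinished as false, so the conversation never signals completion.
; The event graph and construction script add no logic of their own.
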(fn `GetNextDialogue`
  (returns (Text :type String) (hasFinished :type Boolean))
  (bind (_dialogue _dialogueindex) (break `/Game/DialogueSystem/Dialogue` (`self.Dialogue`)))
  (if (not (< _dialogueindex (`KismetArrayLibrary.Array_Length` _dialogue)))
    (`self.ResetDialogue`))
  (`/Engine/EditorBlueprintResources/StandardMacros.IncrementInt` _dialogueindex
    (:`  `
      (return (`|GetArrayItem` _dialogue (- _dialogueindex 1)) false))))

(fn `UserConstructionScript`
  (`parent.UserConstructionScript`))